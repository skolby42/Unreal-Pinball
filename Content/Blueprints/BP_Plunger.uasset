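; Pinball plunger actor that pulls back while charging and moves on release, with a launch sound if a ball is on it.
; ChargePlunger plays a timeline that lerps the mesh along local Y, and StopCharge halts it, then moves the mesh over ReleaseTime.
; Ball overlap sets the flag gating the sound, which clears on release; no impulse is applied here.
; GetBallSpawnLocation converts BallLocation to world space.
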(event `self.ReceiveActorBeginOverlap`
  (params (OtherActor :type "Actor Object Reference"))
  (cast `/Game/Blueprints/BP_Ball` OtherActor)
  (set `self.BallOnPlunger` true))

(event `ChargePlunger`
  (bind (_direction _chargealpha) (`Timeline|ChargeTimeline` :!via `PlayFromStart` :!label _label)
    (:`Update`
      (`SceneComponent.K2_SetRelativeLocation` (`self.PlungerMesh`) (`KismetMathLibrary.VLerp` (0.0 0.0 0.0) (0.0 125.0 0.0) _chargealpha) false false))))

(event `StopCharge`
  (`|ExecutionSequence`
    (:`then_0`
      (goto _label :!via `Stop`))
    (:`then_1`
      (if (`self.BallOnPlunger`)
        (`GameplayStatics.SpawnSoundAttached` "/Game/Assets/Sounds/Pinball_BallLaunch_Cue.Pinball_BallLaunch_Cue" (`self.PlungerMesh`) "None" (0.0 0.0 0.0) (struct) "KeepRelativeOffset" false 1.0 1.0 0.0 null null))
      (`KismetSystemLibrary.MoveComponentTo` (`self.PlungerMesh`) (0.0 0.0 0.0) (struct) false false (`self.ReleaseTime`))
      (set `self.BallOnPlunger` false))))

(fn `GetBallSpawnLocation`
  (returns (BallSpawnLoc :type "Vector Structure"))
  (return (`KismetMathLibrary.TransformLocation` (`self.GetTransform`) (`self.BallLocation`))))

(fn `UserConstructionScript`)