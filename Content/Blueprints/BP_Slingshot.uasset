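; BP_Slingshot is a pinball slingshot bumper that kicks the ball away on contact and awards score.
; When a BP_Ball overlaps the capsule, it plays a kickout sound, adds points through the PinballGameMode and applies an impulse along the capsule's forward vector, scaled by ImpulseMultiplier.
; A timeline then animates the band's bounce through the PercentOut parameter of a dynamic material created in the construction script.
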(event `self.ReceiveActorBeginOverlap`
  (params (OtherActor :type "Actor Object Reference")))

(event `self.Capsule.OnComponentBeginOverlap`
  (params (OverlappedComponent :type "PrimitiveComponent Object Reference") (OtherActor :type "Actor Object Reference") (OtherComp :type "PrimitiveComponent Object Reference") (OtherBodyIndex :type Integer) (bFromSweep :type Boolean) (SweepResult :type "HitResult Structure (by ref)"))
  (bind _asbp_ball (cast `/Game/Blueprints/BP_Ball` OtherActor))
  (bind _aspinball_game_mode (cast `/Game/Blueprints/PinballGameMode` (`GameplayStatics.GetGameMode`))
    (:`then`
      (`GameplayStatics.SpawnSoundAttached` "/Game/Assets/Sounds/Pinball_BallKickout_Cue.Pinball_BallKickout_Cue" (`self.Capsule`) "None" (0.0 0.0 0.0) (struct) "KeepRelativeOffset" false 1.0 1.0 0.0 null null)
      (`/Game/Blueprints/PinballGameMode.AddScore` _aspinball_game_mode 20.0))
    (:`CastFailed`
      _))
  (`PrimitiveComponent.AddImpulse` (`/Game/Blueprints/BP_Ball.Ball` _asbp_ball) (* (`SceneComponent.GetForwardVector` (`self.Capsule`)) (`self.ImpulseMultiplier`)) "None" false)
  (bind (_direction _bounce) (`Timeline|Timeline_0` :!via `PlayFromStart`)
    (:`Update`
      (bind _asmaterial_instance_dynamic (cast `MaterialInstanceDynamic` (`PrimitiveComponent.GetMaterial` (`self.SlingshotBandMesh`) 2)))
      (`MaterialInstanceDynamic.SetScalarParameterValue` _asmaterial_instance_dynamic "PercentOut" _bounce))))

(fn `UserConstructionScript`
  (`PrimitiveComponent.CreateDynamicMaterialInstance` (`self.SlingshotBandMesh`) 2 null "None"))