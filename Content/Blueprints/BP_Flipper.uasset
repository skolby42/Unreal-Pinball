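; Pinball flipper actor that swings up and back as a left or right paddle according to FlipType.
; The construction script picks mirrored start and end rotations, applies the start pose, and flips the X scale for right flippers.
; Flip and Flop events move the Flipper component between those rotations over FlipTime.
; Flip also plays an attached sound, but its switch is fixed to Left, so the left cue always plays.
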(event `self.ReceiveBeginPlay`)

(event `Flip`
  (bind _flipper (`self.Flipper`))
  (switch `/Game/Blueprints/FlipType` "NewEnumerator0"
    (:`NewEnumerator0`
      (`GameplayStatics.SpawnSoundAttached` "/Game/Assets/Sounds/Pinball_FlipperLeft_Cue.Pinball_FlipperLeft_Cue" _flipper "None" (0.0 0.0 0.0) (struct) "KeepRelativeOffset" false 1.0 1.0 0.0 null null))
    (:`NewEnumerator1`
      (`GameplayStatics.SpawnSoundAttached` null _flipper "None" (0.0 0.0 0.0) (struct) "KeepRelativeOffset" false 1.0 1.0 0.0 null null)))
  (`KismetSystemLibrary.MoveComponentTo` (`self.Flipper`) (0.0 0.0 0.0) (`self.EndRotation`) false false (`self.FlipTime`)))

(event `Flop`
  (`KismetSystemLibrary.MoveComponentTo` (`self.Flipper`) (0.0 0.0 0.0) (`self.StartRotation`) false false (`self.FlipTime`)))

(fn `UserConstructionScript`
  (set `self.StartRotation` (select `/Game/Blueprints/FlipType` (`self.FlipType`) :`NewEnumerator0` (struct :`Yaw` 20.0) :`NewEnumerator1` (struct :`Yaw` -20.0) :!type "Rotator Structure"))
  (set `self.EndRotation` (select `/Game/Blueprints/FlipType` (`self.FlipType`) :`NewEnumerator0` (struct :`Yaw` -20.0) :`NewEnumerator1` (struct :`Yaw` 20.0) :!type "Rotator Structure"))
  (`SceneComponent.K2_SetRelativeRotation` (`self.Flipper`) (`self.StartRotation`) false false)
  (switch `/Game/Blueprints/FlipType` (`self.FlipType`)
    (:`NewEnumerator1`
      (`SceneComponent.SetRelativeScale3D` (`self.Flipper`) (-1.0 1.0 1.0)))))