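; Zone actor that steers physics balls (BP_Ball) inside it along the axis of its Arrow component.
; Each Tick, it converts every overlapping ball's velocity into the arrow's local space.
; It interpolates that velocity at AccellSpeed toward pure X-axis motion capped at a fixed maximum, damping sideways and vertical drift without raising slower forward speeds.
; The result returns to world space as the ball's physics linear velocity.
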(event `self.ReceiveTick`
  (params (DeltaSeconds :type "Float (single-precision)"))
  (bind _returnvalue (`SceneComponent.K2_GetComponentToWorld` (`self.Arrow`)))
  (for _array_element (`self.GetOverlappingActors` null)
    (bind _asbp_ball (cast `/Game/Blueprints/BP_Ball` _array_element))
    (bind _returnvalue_2 (`KismetMathLibrary.InverseTransformDirection` _returnvalue (`self.GetVelocity` _array_element)))
    (`PrimitiveComponent.SetPhysicsLinearVelocity` (`/Game/Blueprints/BP_Ball.Ball` _asbp_ball) (`KismetMathLibrary.TransformDirection` _returnvalue (`KismetMathLibrary.VInterpTo` _returnvalue_2 (`KismetMathLibrary.MakeVector` (`KismetMathLibrary.FMin` (.x _returnvalue_2) 800.0)) (`GameplayStatics.GetWorldDeltaSeconds`) (`self.AccellSpeed`))) false "None")))

(fn `UserConstructionScript`)